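; Behavior tree decorator for AI that gates a branch on the distance between the controlled pawn and the player.
; It casts its owner to AIcont and reads the player actor from a Blackboard key.
; Despite the asset name "close", the check passes when that distance is at or beyond the Move threshold, and fails if the cast fails.
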(fn `PerformConditionCheck`
  (params (OwnerActor :type "Actor Object Reference"))
  (returns (ReturnValue :type Boolean))
  (bind _asaicont (cast `/Game/Blueprints/AI/AIcont` OwnerActor))
  (set `self.AIcont` _asaicont)
  (return (>= (`KismetMathLibrary.VSize` (- (`Actor.K2_GetActorLocation` (`BTFunctionLibrary.GetBlackboardValueAsActor` (`self.player`))) (`Actor.K2_GetActorLocation` (`Controller.K2_GetPawn` (`self.AIcont`))))) (`self.move`))))