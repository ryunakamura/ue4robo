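; Behavior tree node that detects nearby game characters for an AI and records them in the blackboard.
; On tick it caches the owning AI controller, then runs a debug-drawn multi-sphere object trace around the controlled pawn.
; Each hit that casts to gamecharacter overwrites the Traget object key and the Playerlook location key, so the last such hit wins.
; The Cloop event is an empty stub.
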(event `Cloop`
  (goto _label :!via `Break`))

(event `self.ReceiveTick`
  (params (OwnerActor :type "Actor Object Reference") (DeltaSeconds :type "Float (single-precision)"))
  (if (== (`self.AIcont`) null)
    (bind _asaicont (cast `/Game/Blueprints/AI/AIcont` OwnerActor))
    (set `self.AIcont` _asaicont))
  (bind _output_get (set `self.mylocation` (`Actor.K2_GetActorLocation` (`Controller.K2_GetPawn` (`self.AIcont`)))))
  (bind (_outhits _returnvalue) (`KismetSystemLibrary.SphereTraceMultiForObjects` _output_get (+ _output_get (0.0 0.0 10.0)) 800.0 (`self.ser`) false (`self.else`) "ForDuration"))
  (if _returnvalue
    (for _index (range (+ (`KismetArrayLibrary.Array_LastIndex` _outhits) 1)) :!label _label
      (bind _asgamecharacter (cast `/Game/Blueprints/gamecharacter` (`.HitActor` (`GameplayStatics.BreakHitResult` (`KismetArrayLibrary.Array_Get` _outhits _index)))))
      (`BTFunctionLibrary.SetBlackboardValueAsObject` (`self.traget`) _asgamecharacter)
      (`BTFunctionLibrary.SetBlackboardValueAsVector` (`self.playerlook`) (`Actor.K2_GetActorLocation` _asgamecharacter)))))