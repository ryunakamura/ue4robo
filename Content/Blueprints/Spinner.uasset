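; Spinner is an actor with a Cube component that spins continuously and changes material while reacting to overlaps.
; Tick adds a fixed one-degree yaw step to the cube's relative rotation each frame, without delta-time scaling, so speed depends on frame rate.
; Any actor overlap beginning switches the cube to a clay brick material, and any overlap ending sets it to CubeMaterial.
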(event `self.ReceiveBeginPlay`)

(event `self.ReceiveActorBeginOverlap`
  (params (OtherActor :type "Actor Object Reference"))
  (`PrimitiveComponent.SetMaterial` (`self.Cube`) 0 "/Game/StarterContent/Materials/M_Brick_Clay_Beveled.M_Brick_Clay_Beveled"))

(event `OnActorEndOverlap_イベント_0`
  (params (OtherActor :type "Actor Object Reference")))

(event `self.ReceiveActorEndOverlap`
  (params (OtherActor :type "Actor Object Reference"))
  (`PrimitiveComponent.SetMaterial` (`self.Cube`) 0 "/Game/Geometry/Meshes/CubeMaterial.CubeMaterial"))

(event `self.ReceiveTick`
  (params (DeltaSeconds :type "Float (single-precision)"))
  (bind _cube (`self.Cube`))
  ;[1 1 1] 回転
  (`SceneComponent.K2_SetRelativeRotation` _cube (`KismetMathLibrary.MakeRotator` (.roll (`SceneComponent.RelativeRotation` _cube)) (.pitch (`SceneComponent.RelativeRotation` _cube)) (+ (.yaw (`SceneComponent.RelativeRotation` _cube)) 1.0)) false false))

(fn `UserConstructionScript`)