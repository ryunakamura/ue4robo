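; Player character Blueprint with jump and forward/right movement input, plus montage playback and socket debug drawing.
; Axis inputs feed movement vectors along the actor's own forward and right directions into CharacterMovement.
; BeginPlay sets a short timer by function name that plays a test montage.
; While Bcanpan is true, Tick draws a debug sphere at the mesh's "pan" socket.
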(event `InputAction|Jump`
  (params (Key :type "Key Structure" :default "AnyKey"))
  ;[1 1 1] ジャンプ
  (:`Pressed`
    (`self.Jump`)))

(event `InputAxis|MoveForward`
  (params (AxisValue :type "Float (single-precision)"))
  ;[1 1 1] 前
  (`PawnMovementComponent.AddInputVector` (`self.CharacterMovement`) (* (`self.GetActorForwardVector`) AxisValue) false))

(event `self.ReceiveBeginPlay`
  (`KismetSystemLibrary.K2_SetTimer` self "mont" 1.0))

(event `self.ReceiveActorBeginOverlap`
  (params (OtherActor :type "Actor Object Reference")))

(event `mont`
  (`self.PlayAnimMontage` "/Game/Mannequin/Animations/TestAnimMontage.TestAnimMontage"))

(event `self.ReceiveTick`
  (params (DeltaSeconds :type "Float (single-precision)"))
  (if (`self.Bcanpan`)
    (`KismetSystemLibrary.DrawDebugSphere` (`SceneComponent.GetSocketLocation` (`self.Mesh`) "pan") 16.0 12 (struct :`R` 1.0 :`B` 0.666894 :`A` 1.0) 1.0)))

(event `InputAxis|MoveRight`
  (params (AxisValue :type "Float (single-precision)"))
  ;[1 1 1] 右
  (`PawnMovementComponent.AddInputVector` (`self.CharacterMovement`) (* (`self.GetActorRightVector`) AxisValue) false))

(fn `UserConstructionScript`)